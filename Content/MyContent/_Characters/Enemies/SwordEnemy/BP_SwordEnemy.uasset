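; Sword enemy character Blueprint that binds its overhead health bar and flags landings after heavy hits.
; On BeginPlay it casts the HealthBar widget to WBP_EnemyHealthBar and sets itself as that widget's owning enemy.
; Landing while in the DamagedHeavy combat state briefly raises LandedFromLaunch, then clears it after a short delay.
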(event `self.ReceiveBeginPlay`
  (bind _aswbp_enemy_health_bar (cast `/Game/MyContent/UserInterface/WBP_EnemyHealthBar` (`WidgetComponent.GetWidget` (`self.HealthBar`))))
  (`/Engine/EditorBlueprintResources/StandardMacros.IsValid` _aswbp_enemy_health_bar
    (:`Is Valid`
      (set `/Game/MyContent/UserInterface/WBP_EnemyHealthBar.OwningEnemy` self _aswbp_enemy_health_bar))))

(event `self.OnLanded`
  (params (Hit :type "HitResult Structure (by ref)"))
  (if (`|EnumEquality` (`self.CombatState`) "COMBAT_DamagedHeavy")
    (set `self.bLandedFromLaunch` true)
    (`KismetSystemLibrary.Delay` 0.2)
    (set `self.bLandedFromLaunch` false)))

(fn `UserConstructionScript`)