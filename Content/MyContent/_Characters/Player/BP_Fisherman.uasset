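; BP_Fisherman is the player character Blueprint, handling the grapple move and landing from a heavy-damage launch.
; Grapple prepares the rope, then a timeline lerps the player's position, finishing by consuming and resetting the rope.
; Each timeline update runs a capsule overlap at the player's position and launches the first hit actor if it is a BP_SpearEnemy.
; Landing while in DamagedHeavy briefly pulses LandedFromLaunch.
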(event `self.OnLanded`
  (params (Hit :type "HitResult Structure (by ref)"))
  (if (`|EnumEquality` (`self.CombatState`) "COMBAT_DamagedHeavy")
    (set `self.bLandedFromLaunch` true)
    (`KismetSystemLibrary.Delay` 0.2)
    (set `self.bLandedFromLaunch` false)))

(event `self.Grapple`
  (bind _capsulecomponent (`self.CapsuleComponent`))
  (`self.PrepareGrapple`)
  (bind (_direction _track) (`Timeline|GrappleTimeline` :!via `PlayFromStart`)
    (:`Update`
      (`self.LerpPlayerPosition` _track)
      (bind _outactors (`KismetSystemLibrary.CapsuleOverlapActors` (`self.K2_GetActorLocation`) (`CapsuleComponent.CapsuleRadius` _capsulecomponent) (`CapsuleComponent.CapsuleHalfHeight` _capsulecomponent) (`|MakeArray` "ObjectTypeQuery7" :!type "EObjectTypeQuery Enum") null (`|MakeArray` self :!type "Actor Object Reference")))
      (if (> (`KismetArrayLibrary.Array_Length` _outactors) 0)
        (bind _asbp_spear_enemy (cast `/Game/MyContent/_Characters/Enemies/SpearEnemy/BP_SpearEnemy` (`|GetArrayItem` _outactors)))
        (`self.LaunchEnemy` _asbp_spear_enemy)))
    (:`Finished`
      (`self.ConsumeRope`)
      (`self.ResetRope`))))

(fn `UserConstructionScript`)